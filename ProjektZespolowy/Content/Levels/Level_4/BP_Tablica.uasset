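; BP_Tablica is an interactive Level 4 board that presents a two-part task through the Part1 and Part2 widget components.
; Interaction toggles a fixed camera view via FlipFlop, hiding the first-person mesh and enabling cursor, UI input and widget collision.
; Part1 shows until its widget reports Passed, then Part2 takes over.
; Once Part2 is passed, interacting only runs the exit path, restoring game-only input.
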(event `self.ReceiveBeginPlay`
  (bind _aswbp_level_4part_ii (cast `/Game/LevelWidgets/LEVEL4/WBP_Level4PartII` (`WidgetComponent.GetWidget` (`self.Part2`))))
  (set `self.SecondWidget` _aswbp_level_4part_ii)
  (bind _aswbp_level_4part_i (cast `/Game/LevelWidgets/LEVEL4/WBP_Level4PartI` (`WidgetComponent.GetWidget` (`self.Part1`))))
  (set `self.FirstWidget` _aswbp_level_4part_i))

(event `self.BeginInteraction`
  (bind _returnvalue (`GameplayStatics.GetPlayerCharacter` 0))
  (bind _returnvalue_2 (`GameplayStatics.GetPlayerController` 0))
  (bind _returnvalue_3 (`GameplayStatics.GetPlayerController` 0))
  (bind _part1 (`self.Part1`))
  (bind _part2 (`self.Part2`))
  (bind _part1_2 (`self.Part1`))
  (bind _part2_2 (`self.Part2`))
  (bind _part1_3 (`self.Part1`))
  (if (`/Game/LevelWidgets/LEVEL4/WBP_Level4PartII.Passed?` (`self.SecondWidget`))
    (message `/Game/Interactions/BPI_Interaction.Camera_Adjust_Off` _returnvalue :!label _label)
    (bind _firstpersonmesh (`/Game/FirstPerson/Blueprints/BP_FirstPersonCharacter.FirstPersonMesh` (stale _asbp_first_person_character)))
    (`SceneComponent.SetVisibility` _firstpersonmesh true false)
    (if (`/Game/LevelWidgets/LEVEL4/WBP_Level4PartI.Passed?` (`self.FirstWidget`))
      (`SceneComponent.SetVisibility` _part2_2 false false)
      (set `PlayerController.bShowMouseCursor` false _returnvalue_2)
      (`WidgetBlueprintLibrary.SetInputMode_GameOnly` _returnvalue_2)
      (`PrimitiveComponent.SetCollisionEnabled` _part2_2 "NoCollision")
      (`SceneComponent.SetVisibility` _part1_2 false false)
      (`PrimitiveComponent.SetCollisionEnabled` _part1_2 "NoCollision")
      (else
        (`SceneComponent.SetVisibility` _part1_3 false false)
        (set `PlayerController.bShowMouseCursor` false _returnvalue_2)
        (`WidgetBlueprintLibrary.SetInputMode_GameOnly` _returnvalue_2)
        (`PrimitiveComponent.SetCollisionEnabled` _part1_3 "NoCollision")))
    (else
      (bind _asbp_first_person_character (cast `/Game/FirstPerson/Blueprints/BP_FirstPersonCharacter` _returnvalue))
      (`/Engine/EditorBlueprintResources/StandardMacros.FlipFlop`
        (:`A`
          (message `/Game/Interactions/BPI_Interaction.Camera_Adjust_On` _returnvalue (`KismetMathLibrary.MakeVector` -10.0 400.0 200.0) (`KismetMathLibrary.MakeRotator` 0.0 0.0 90.0))
          (`SceneComponent.SetVisibility` _firstpersonmesh false false)
          (if (`/Game/LevelWidgets/LEVEL4/WBP_Level4PartI.Passed?` (`self.FirstWidget`))
            (`SceneComponent.SetVisibility` _part2 true false)
            (set `PlayerController.bShowMouseCursor` true _returnvalue_3)
            (`WidgetBlueprintLibrary.SetInputMode_GameAndUIEx` _returnvalue_3 null "DoNotLock" false)
            (`PrimitiveComponent.SetCollisionEnabled` _part2 "QueryAndPhysics")
            (else
              (`SceneComponent.SetVisibility` _part1 true false)
              (set `PlayerController.bShowMouseCursor` true _returnvalue_3)
              (`WidgetBlueprintLibrary.SetInputMode_GameAndUIEx` _returnvalue_3 null "DoNotLock" false)
              (`PrimitiveComponent.SetCollisionEnabled` _part1 "QueryAndPhysics"))))
        (:`B`
          (goto _label))))))

(fn `UserConstructionScript`)