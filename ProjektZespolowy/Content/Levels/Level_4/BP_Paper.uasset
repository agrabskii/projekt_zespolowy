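; BP_Paper is an interactable paper in Level 4 that toggles a close-up view of its TruthFalse component.
; Interaction only works once the SecondWidget on BP_Tablica reports Passed.
; A FlipFlop alternates between moving the player camera to a hardcoded pose with TruthFalse visible, collidable and mouse input enabled, and restoring the camera and game-only input with it hidden.
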(event `self.BeginInteraction`
  (bind _returnvalue (`GameplayStatics.GetPlayerCharacter` 0))
  (bind _returnvalue_2 (`GameplayStatics.GetPlayerController` 0))
  (bind _truthfalse (`self.TruthFalse`))
  (bind _returnvalue_3 (`GameplayStatics.GetActorOfClass` "/Game/Levels/Level_4/BP_Tablica.BP_Tablica_C"))
  (if (`/Game/LevelWidgets/LEVEL4/WBP_Level4PartII.Passed?` (`/Game/Levels/Level_4/BP_Tablica.SecondWidget` _returnvalue_3))
    (cast `/Game/FirstPerson/Blueprints/BP_FirstPersonCharacter` _returnvalue)
    (`/Engine/EditorBlueprintResources/StandardMacros.FlipFlop`
      (:`A`
        (message `/Game/Interactions/BPI_Interaction.Camera_Adjust_On` _returnvalue (`KismetMathLibrary.MakeVector` -155.890967 -28.10636 150.0) (`KismetMathLibrary.MakeRotator` -57.3 -90.0))
        (`SceneComponent.SetVisibility` _truthfalse true false)
        (set `PlayerController.bShowMouseCursor` true _returnvalue_2)
        (`WidgetBlueprintLibrary.SetInputMode_GameAndUIEx` _returnvalue_2 null "DoNotLock" false)
        (`PrimitiveComponent.SetCollisionEnabled` _truthfalse "QueryAndPhysics"))
      (:`B`
        (message `/Game/Interactions/BPI_Interaction.Camera_Adjust_Off` _returnvalue)
        (`SceneComponent.SetVisibility` _truthfalse false false)
        (set `PlayerController.bShowMouseCursor` false _returnvalue_2)
        (`WidgetBlueprintLibrary.SetInputMode_GameOnly` _returnvalue_2)
        (`PrimitiveComponent.SetCollisionEnabled` _truthfalse "NoCollision")))))

(fn `UserConstructionScript`)