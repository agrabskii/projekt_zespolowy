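; BP_Sala2 is the room controller for Level 2 that advances the game to Level 3 once three completion flags are set.
; Every Tick it prints Comp1, Comp2 and Comp3 as debug text and checks whether all three are true.
; When they are, it hides the mouse cursor, switches input to game-only and opens L_Level3.
; The flags are only read here, never set.
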(event `self.ReceiveBeginPlay`)

(event `self.ReceiveTick`
  (params (DeltaSeconds :type "Float (single-precision)"))
  (bind _returnvalue (`GameplayStatics.GetPlayerController` 0))
  (bind _comp3 (`self.Comp3`))
  (bind _comp1 (`self.Comp1`))
  (bind _comp2 (`self.Comp2`))
  (`KismetSystemLibrary.PrintText` (`KismetTextLibrary.Conv_BoolToText` _comp1))
  (`KismetSystemLibrary.PrintText` (`KismetTextLibrary.Conv_BoolToText` _comp2))
  (`KismetSystemLibrary.PrintText` (`KismetTextLibrary.Conv_BoolToText` _comp3))
  (if (and (and _comp1 _comp2) _comp3)
    (set `PlayerController.bShowMouseCursor` false _returnvalue)
    (`WidgetBlueprintLibrary.SetInputMode_GameOnly` _returnvalue)
    (`GameplayStatics.OpenLevelBySoftObjectPtr` "/Game/Levels/Level_3/L_Level3.L_Level3")))

(fn `UserConstructionScript`)