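; BP_Paper10 is an interactable paper in Level 10 that shows a question when the player interacts with it.
; Each interaction toggles via a FlipFlop: the first tells the first-person character to move its camera to a fixed close-up and reveals the question component with collision, mouse cursor and Game-and-UI input.
; The next restores the camera, hides and disables the question, and returns to game-only input.
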(event `self.BeginInteraction`
  (bind _returnvalue (`GameplayStatics.GetPlayerCharacter` 0))
  (bind _returnvalue_2 (`GameplayStatics.GetPlayerController` 0))
  (bind _1question (`self.1Question`))
  (cast `/Game/FirstPerson/Blueprints/BP_FirstPersonCharacter` _returnvalue)
  (`/Engine/EditorBlueprintResources/StandardMacros.FlipFlop`
    (:`A`
      (message `/Game/Interactions/BPI_Interaction.Camera_Adjust_On` _returnvalue (`KismetMathLibrary.MakeVector` -60.906027 434.797042 159.568747) (`KismetMathLibrary.MakeRotator` -78.0 -90.0))
      (`SceneComponent.SetVisibility` _1question true false)
      (set `PlayerController.bShowMouseCursor` true _returnvalue_2)
      (`WidgetBlueprintLibrary.SetInputMode_GameAndUIEx` _returnvalue_2 null "DoNotLock" false)
      (`PrimitiveComponent.SetCollisionEnabled` _1question "QueryAndPhysics"))
    (:`B`
      (message `/Game/Interactions/BPI_Interaction.Camera_Adjust_Off` _returnvalue)
      (`SceneComponent.SetVisibility` _1question false false)
      (set `PlayerController.bShowMouseCursor` false _returnvalue_2)
      (`WidgetBlueprintLibrary.SetInputMode_GameOnly` _returnvalue_2)
      (`PrimitiveComponent.SetCollisionEnabled` _1question "NoCollision"))))

(fn `UserConstructionScript`)