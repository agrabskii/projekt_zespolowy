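; BP_Monitor10 is an interactable monitor in Level 10 that hosts the WBP_Zadanie2 task widget.
; Interaction and the widget's exit button share one FlipFlop, so each trigger toggles between entering and leaving the monitor view.
; Entering messages the player character to move its camera to a hardcoded transform and enables cursor and Game and UI input.
; Leaving releases the camera and restores game-only input.
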(event `self.ReceiveBeginPlay`
  (bind _aswbp_zadanie_2 (cast `/Game/Levels/Level_10/Components/WBP_Zadanie2` (`WidgetComponent.GetWidget` (`self.Zad2`))))
  (add `Button.OnClicked` (`/Game/Levels/Level_10/Components/WBP_Zadanie2.Exit_Button` _aswbp_zadanie_2) (delegate `GoOut`)))

(event `GoOut`
  (bind _returnvalue (`GameplayStatics.GetPlayerCharacter` 0))
  (bind _returnvalue_2 (`GameplayStatics.GetPlayerController` 0))
  (`/Engine/EditorBlueprintResources/StandardMacros.FlipFlop` :!label _label
    (:`A`
      (message `/Game/Interactions/BPI_Interaction.Camera_Adjust_On` _returnvalue (`KismetMathLibrary.MakeVector` -190.334523 -281.78375 160.66165) (`KismetMathLibrary.MakeRotator` 0.0 -5.0 180.0))
      (set `PlayerController.bShowMouseCursor` true _returnvalue_2)
      (`WidgetBlueprintLibrary.SetInputMode_GameAndUIEx` _returnvalue_2 null "DoNotLock" false))
    (:`B`
      (message `/Game/Interactions/BPI_Interaction.Camera_Adjust_Off` _returnvalue)
      (set `PlayerController.bShowMouseCursor` false _returnvalue_2)
      (`WidgetBlueprintLibrary.SetInputMode_GameOnly` _returnvalue_2))))

(event `self.BeginInteraction`
  (goto _label))

(fn `UserConstructionScript`)