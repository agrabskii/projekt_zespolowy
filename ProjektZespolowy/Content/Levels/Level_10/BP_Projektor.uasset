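; BP_Projektor is an interactable projector in Level 10 that reveals content once the first task is answered correctly.
; On BeginInteraction it reads the Correct flag from the WBP_Zadanie1 widget on BP_Paper10's question component.
; If correct, it makes the BP_Screen plane, every BP_MonitorNoise mesh and the Zad2 component of BP_Monitor10 visible, finding each actor by class lookup.
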(event `self.BeginInteraction`
  (bind _returnvalue (`GameplayStatics.GetActorOfClass` "/Game/Levels/Level_10/BP_Paper10.BP_Paper10_C"))
  (bind _aswbp_zadanie_1 (cast `/Game/Levels/Level_10/Components/WBP_Zadanie1` (`WidgetComponent.GetWidget` (`/Game/Levels/Level_10/BP_Paper10.1Question` _returnvalue))))
  (if (`/Game/Levels/Level_10/Components/WBP_Zadanie1.correct?` _aswbp_zadanie_1)
    (bind _returnvalue_2 (`GameplayStatics.GetActorOfClass` "/Game/Levels/Level_10/ProjectorShader/BP_Screen.BP_Screen_C"))
    (`SceneComponent.SetVisibility` (`/Game/Levels/Level_10/ProjectorShader/BP_Screen.Plane` _returnvalue_2) true false)
    (bind _outactors (`GameplayStatics.GetAllActorsOfClass` "/Game/Levels/Level_10/MonitorNoiseShader/BP_MonitorNoise.BP_MonitorNoise_C"))
    (for _array_element _outactors
      (`SceneComponent.SetVisibility` (`/Game/Levels/Level_10/MonitorNoiseShader/BP_MonitorNoise.StaticMesh` _array_element) true false))
    (bind _returnvalue_3 (`GameplayStatics.GetActorOfClass` "/Game/Levels/Level_10/BP_Monitor10.BP_Monitor10_C"))
    (`SceneComponent.SetVisibility` (`/Game/Levels/Level_10/BP_Monitor10.Zad2` _returnvalue_3) true false)))

(fn `UserConstructionScript`)