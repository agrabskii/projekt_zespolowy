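; BP_Level7_Instructions is an interactable Level 7 instructions actor that stays hidden until its Zaliczonekompyzkartki counter reaches four.
; Tick checks the counter every frame to reveal the actor; nothing in this graph changes the count.
; Once unlocked, each interaction toggles through a FlipFlop between blending the view to this actor with movement and look input disabled, and returning camera and controls to the player.
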(event `self.ReceiveBeginPlay`
  (`self.SetActorHiddenInGame` true))

(event `self.ReceiveTick`
  (params (DeltaSeconds :type "Float (single-precision)"))
  (if (>= (`self.Zaliczonekompyzkartki`) 4)
    (`self.SetActorHiddenInGame` false)))

(event `self.BeginInteraction`
  (bind _returnvalue (`GameplayStatics.GetPlayerCharacter` 0))
  (bind _charactermovement (`Character.CharacterMovement` _returnvalue))
  (bind _returnvalue_2 (`PlayerState.GetPlayerController` (`Pawn.PlayerState` _returnvalue)))
  (if (>= (`self.Zaliczonekompyzkartki`) 4)
    (`/Engine/EditorBlueprintResources/StandardMacros.FlipFlop`
      (:`A`
        (`PlayerController.SetViewTargetWithBlend` _returnvalue_2 self 1.0 "VTBlend_Linear" 0.0 false)
        (`CharacterMovementComponent.DisableMovement` _charactermovement)
        (`Controller.SetIgnoreLookInput` _returnvalue_2 true))
      (:`B`
        (`PlayerController.SetViewTargetWithBlend` _returnvalue_2 (`GameplayStatics.GetPlayerCharacter` 0) 1.0 "VTBlend_Linear" 0.0 false)
        (`CharacterMovementComponent.SetMovementMode` _charactermovement "MOVE_Walking" 0)
        (`Controller.SetIgnoreLookInput` _returnvalue_2 false)))))

(fn `UserConstructionScript`)