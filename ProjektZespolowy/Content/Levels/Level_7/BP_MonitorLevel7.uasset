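; BP_MonitorLevel7 is an interactable monitor for Level 7 that hosts a WBP_MonitorLevel7 widget.
; BeginInteraction passes the monitor's reference to that widget, then a FlipFlop toggles between using and leaving the monitor.
; Using it blends the view to the monitor, shows the cursor, allows UI input and disables character movement.
; Leaving blends back to the character and restores game-only input and walking.
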(event `self.BeginInteraction`
  (bind _returnvalue (`GameplayStatics.GetPlayerCharacter` 0))
  (bind _returnvalue_2 (`GameplayStatics.GetPlayerController` 0))
  (bind _charactermovement (`Character.CharacterMovement` _returnvalue))
  (bind _aswbp_monitor_level_7 (cast `/Game/Levels/Level_7/WBP_MonitorLevel7` (`WidgetComponent.GetUserWidgetObject` (`self.Widget`))))
  (set `/Game/Levels/Level_7/WBP_MonitorLevel7.MonitorRef` self _aswbp_monitor_level_7)
  (`/Engine/EditorBlueprintResources/StandardMacros.FlipFlop`
    (:`A`
      (set `PlayerController.bShowMouseCursor` true _returnvalue_2)
      (`PlayerController.SetViewTargetWithBlend` _returnvalue_2 self 1.0 "VTBlend_Linear" 0.0 false)
      (`WidgetBlueprintLibrary.SetInputMode_GameAndUIEx` _returnvalue_2 null "DoNotLock" false)
      (`CharacterMovementComponent.DisableMovement` _charactermovement))
    (:`B`
      (set `PlayerController.bShowMouseCursor` false _returnvalue_2)
      (`PlayerController.SetViewTargetWithBlend` _returnvalue_2 _returnvalue 1.0 "VTBlend_Linear" 0.0 false)
      (`WidgetBlueprintLibrary.SetInputMode_GameOnly` _returnvalue_2)
      (`CharacterMovementComponent.SetMovementMode` _charactermovement "MOVE_Walking" 0))))

(fn `UserConstructionScript`)