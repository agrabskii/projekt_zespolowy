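; BP_Door_With_Lock is a door variant fitted with a combination padlock as the Lock child actor.
; Its SetOdp event casts that child actor to BP_Klodka_Szyfrowa and forwards four answer values (Odp1 to Odp4) plus LevelClass to the padlock's own SetOdp.
; The construction script only calls its parent, and no unlock or opening logic lives in this Blueprint.
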(event `SetOdp`
  (bind _asbp_klodka_szyfrowa (cast `/Game/Levels/Level_6/BP_Klodka_Szyfrowa` (`ChildActorComponent.ChildActor` (`self.Lock`))))
  (`/Game/Levels/Level_6/BP_Klodka_Szyfrowa.SetOdp` _asbp_klodka_szyfrowa (`self.Odp 1`) (`self.Odp 2`) (`self.Odp 3`) (`self.Odp 4`) (`self.LevelClass`)))

(fn `UserConstructionScript`
  (`parent.UserConstructionScript`))