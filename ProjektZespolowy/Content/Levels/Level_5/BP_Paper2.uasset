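; BP_Paper2 is an interactable paper in Level 5 that toggles an on-screen WB_Kartka2 widget when the player interacts with it.
; BeginInteraction calls the parent, then a FlipFlop alternates between showing and hiding the widget along with the mouse cursor, switching between Game-and-UI and Game-only input.
; Each opening creates a new widget after a BP_FirstPersonCharacter cast check, while closing only hides it without removing it from the viewport.
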(event `self.BeginInteraction`
  (bind _returnvalue (`GameplayStatics.GetPlayerController` 0))
  (bind _returnvalue_2 (`GameplayStatics.GetPlayerController` 0))
  (bind _kartka_widget (`self.Kartka Widget`))
  (bind _kartka_widget_2 (`self.Kartka Widget`))
  (`parent.BeginInteraction`)
  (`/Engine/EditorBlueprintResources/StandardMacros.FlipFlop`
    (:`A`
      (cast `/Game/FirstPerson/Blueprints/BP_FirstPersonCharacter` (`GameplayStatics.GetPlayerCharacter` 0))
      (bind _returnvalue_3 (`|CreateWidget` "/Game/LevelWidgets/Level5/WB_Kartka2.WB_Kartka2_C" (`GameplayStatics.GetPlayerController` 0)))
      (bind _output_get (set `self.Kartka Widget` _returnvalue_3))
      (`Border.SetBrushColor` (`/Game/LevelWidgets/Level5/WB_Kartka2.Border_89` _output_get) (struct :`R` 1.0 :`G` 1.0 :`B` 1.0 :`A` 1.0))
      (`UserWidget.AddToViewport` _kartka_widget 0)
      (`Widget.SetVisibility` _kartka_widget "Visible")
      (set `PlayerController.bShowMouseCursor` true _returnvalue)
      (`WidgetBlueprintLibrary.SetInputMode_GameAndUIEx` _returnvalue null "DoNotLock" false))
    (:`B`
      (`Border.SetBrushColor` (`/Game/LevelWidgets/Level5/WB_Kartka2.Border_89` _kartka_widget_2) (struct :`R` 1.0 :`G` 1.0 :`B` 1.0))
      (`Widget.SetVisibility` _kartka_widget_2 "Hidden")
      (set `PlayerController.bShowMouseCursor` false _returnvalue_2)
      (`WidgetBlueprintLibrary.SetInputMode_GameOnly` _returnvalue_2))))

(fn `UserConstructionScript`
  (`parent.UserConstructionScript`))