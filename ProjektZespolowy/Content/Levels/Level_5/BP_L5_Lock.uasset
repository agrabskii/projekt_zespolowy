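; BP_L5_Lock is the interactable lock in Level 5 that toggles an on-screen lock widget.
; It extends the parent's BeginInteraction with a FlipFlop that alternates between opening and closing the UI.
; Opening checks the first-person character, creates a new WB_Level5_Lock each time, and enables the cursor with Game and UI input.
; Closing only hides that widget, then restores game-only input without a cursor.
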(event `self.BeginInteraction`
  (bind _returnvalue (`GameplayStatics.GetPlayerController` 0))
  (bind _returnvalue_2 (`GameplayStatics.GetPlayerController` 0))
  (`parent.BeginInteraction`)
  (`/Engine/EditorBlueprintResources/StandardMacros.FlipFlop`
    (:`A`
      (cast `/Game/FirstPerson/Blueprints/BP_FirstPersonCharacter` (`GameplayStatics.GetPlayerCharacter` 0))
      (bind _returnvalue_3 (`|CreateWidget` "/Game/LevelWidgets/Level5/WB_Level5_Lock.WB_Level5_Lock_C" (`GameplayStatics.GetPlayerController` 0)))
      (bind _output_get (set `self.LockWidget` _returnvalue_3))
      (`UserWidget.AddToViewport` _output_get 0)
      (`Widget.SetVisibility` (`self.LockWidget`) "Visible")
      (set `PlayerController.bShowMouseCursor` true _returnvalue)
      (`WidgetBlueprintLibrary.SetInputMode_GameAndUIEx` _returnvalue null "DoNotLock" false))
    (:`B`
      (`Widget.SetVisibility` (`self.LockWidget`) "Hidden")
      (set `PlayerController.bShowMouseCursor` false _returnvalue_2)
      (`WidgetBlueprintLibrary.SetInputMode_GameOnly` _returnvalue_2))))

(fn `UserConstructionScript`
  (`parent.UserConstructionScript`))