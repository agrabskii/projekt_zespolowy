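; BP_Level11_Lock is an interactable lock in Level 11 that opens and closes its own UI widget.
; BeginInteraction calls the parent, then a FlipFlop alternates between opening and closing.
; Opening creates a new WBP_Level11_Lock with a reference to itself, shows the cursor, allows UI input and disables player movement.
; Closing hides the widget without removing it and restores game-only input and walking.
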(event `self.BeginInteraction`
  (bind _returnvalue (`GameplayStatics.GetPlayerController` 0))
  (bind _returnvalue_2 (`GameplayStatics.GetPlayerController` 0))
  (bind _charactermovement (`Character.CharacterMovement` (`GameplayStatics.GetPlayerCharacter` 0)))
  (`parent.BeginInteraction`)
  (`/Engine/EditorBlueprintResources/StandardMacros.FlipFlop`
    (:`A`
      (bind _returnvalue_3 (`|CreateWidget` "/Game/Levels/Level_11/WBP_Level11_Lock.WBP_Level11_Lock_C" (`GameplayStatics.GetPlayerController` 0) self))
      (bind _output_get (set `self.LockWidget` _returnvalue_3))
      (`UserWidget.AddToViewport` _output_get 0)
      (`Widget.SetVisibility` (`self.LockWidget`) "Visible")
      (set `PlayerController.bShowMouseCursor` true _returnvalue)
      (`WidgetBlueprintLibrary.SetInputMode_GameAndUIEx` _returnvalue null "DoNotLock" false)
      (`CharacterMovementComponent.DisableMovement` _charactermovement))
    (:`B`
      (`Widget.SetVisibility` (`self.LockWidget`) "Hidden")
      (set `PlayerController.bShowMouseCursor` false _returnvalue_2)
      (`WidgetBlueprintLibrary.SetInputMode_GameOnly` _returnvalue_2)
      (`CharacterMovementComponent.SetMovementMode` _charactermovement "MOVE_Walking" 0))))

(fn `UserConstructionScript`
  (`parent.UserConstructionScript`))