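; Interactive in-game monitor for Level 11 that hosts a short quiz across three widget components: desktop (Pulpit), Test and result (Wynik).
; BeginInteraction flip-flops between a fixed screen camera with mouse input and normal gameplay; each screen's Exit button calls the same toggle.
; Buttons swap screens via visibility and collision, with CurrentWidget tracking the active one.
; Submit shows the result only when all three hardcoded answers match exactly.
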(event `Exit`
  (`self.BeginInteraction`))

(event `GoToTest`
  (bind _test (`self.Test`))
  (bind _pulpit (`self.Pulpit`))
  (`SceneComponent.SetVisibility` _pulpit false false)
  (`PrimitiveComponent.SetCollisionEnabled` _pulpit "NoCollision")
  (`SceneComponent.SetVisibility` _test true false)
  (`PrimitiveComponent.SetCollisionEnabled` _test "QueryOnly")
  (set `self.Current_Widget` _test))

(event `self.ReceiveBeginPlay`
  (bind _pulpit (`self.Pulpit`))
  (`|ExecutionSequence`
    (:`then_0`
      (`PrimitiveComponent.SetCollisionEnabled` (`self.Test`) "NoCollision")
      (`PrimitiveComponent.SetCollisionEnabled` (`self.Wynik`) "NoCollision")
      (bind _aswbp_pulpit (cast `/Game/Levels/Level_11/Widgets/WBP_Pulpit` (`WidgetComponent.GetWidget` _pulpit)))
      (add `Button.OnClicked` (`/Game/Levels/Level_11/Widgets/WBP_Pulpit.Exit_Button` _aswbp_pulpit) (delegate `Exit`))
      (add `Button.OnClicked` (`/Game/Levels/Level_11/Widgets/WBP_Pulpit.Test` _aswbp_pulpit) (delegate `GoToTest`))
      (set `self.Current_Widget` _pulpit))
    (:`then_1`
      (bind _aswbp_test (cast `/Game/Levels/Level_11/Widgets/WBP_Test` (`WidgetComponent.GetWidget` (`self.Test`))))
      (add `Button.OnClicked` (`/Game/Levels/Level_11/Widgets/WBP_Test.Exit_Button` _aswbp_test) (delegate `Exit`))
      (add `Button.OnClicked` (`/Game/Levels/Level_11/Widgets/WBP_Test.Submit_Button` _aswbp_test) (delegate `CheckAnswersAndGoToResult`)))
    (:`then_2`
      (bind _aswbp_wynik (cast `/Game/Levels/Level_11/Widgets/WBP_Wynik` (`WidgetComponent.GetWidget` (`self.Wynik`))))
      (add `Button.OnClicked` (`/Game/Levels/Level_11/Widgets/WBP_Wynik.Exit_Button` _aswbp_wynik) (delegate `Exit`)))))

(event `CheckAnswersAndGoToResult`
  (bind _test (`self.Test`))
  (bind _wynik (`self.Wynik`))
  (bind _aswbp_test (cast `/Game/Levels/Level_11/Widgets/WBP_Test` (`WidgetComponent.GetWidget` _test)))
  (if (and (== (`KismetTextLibrary.Conv_TextToString` (`EditableText.GetText` (`/Game/Levels/Level_11/Widgets/WBP_Test.ODP1` _aswbp_test))) "ray tracing") (== (`KismetTextLibrary.Conv_TextToString` (`EditableText.GetText` (`/Game/Levels/Level_11/Widgets/WBP_Test.ODP2` _aswbp_test))) "tak") (== (`KismetTextLibrary.Conv_TextToString` (`EditableText.GetText` (`/Game/Levels/Level_11/Widgets/WBP_Test.ODP3` _aswbp_test))) "tak"))
    (`SceneComponent.SetVisibility` _test false false)
    (`PrimitiveComponent.SetCollisionEnabled` _test "NoCollision")
    (`SceneComponent.SetVisibility` _wynik true false)
    (`PrimitiveComponent.SetCollisionEnabled` _wynik "QueryOnly")
    (set `self.Current_Widget` _wynik)))

(event `self.BeginInteraction`
  (bind _returnvalue (`GameplayStatics.GetPlayerCharacter` 0))
  (bind _returnvalue_2 (`GameplayStatics.GetPlayerController` 0))
  (bind _current_widget (`self.Current_Widget`))
  (`KismetSystemLibrary.PrintText` "Interakcja działa")
  (`/Engine/EditorBlueprintResources/StandardMacros.FlipFlop`
    (:`A`
      (message `/Game/Interactions/BPI_Interaction.Camera_Adjust_On` _returnvalue (`KismetMathLibrary.MakeVector` -200.0 -110.0 155.0) (`KismetMathLibrary.MakeRotator` 0.0 -5.0 180.0))
      (set `PlayerController.bShowMouseCursor` true _returnvalue_2)
      (`WidgetBlueprintLibrary.SetInputMode_GameAndUIEx` _returnvalue_2 null "DoNotLock" false)
      (`SceneComponent.SetVisibility` _current_widget true false)
      (`PrimitiveComponent.SetCollisionEnabled` (`self.Current_Widget`) "QueryOnly"))
    (:`B`
      (message `/Game/Interactions/BPI_Interaction.Camera_Adjust_Off` _returnvalue)
      (set `PlayerController.bShowMouseCursor` false _returnvalue_2)
      (`WidgetBlueprintLibrary.SetInputMode_GameOnly` _returnvalue_2)
      (`SceneComponent.SetVisibility` _current_widget false false)
      (`PrimitiveComponent.SetCollisionEnabled` (`self.Current_Widget`) "NoCollision"))))

(fn `UserConstructionScript`)