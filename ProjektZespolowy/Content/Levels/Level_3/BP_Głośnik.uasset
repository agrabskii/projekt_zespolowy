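; Interactable speaker (Głośnik) in Level 3 that opens its own UI widget once the player character's Level3Interacted flag is set.
; The first interaction creates the WB_Level3_Glosnik widget, shows the cursor and switches to Game and UI input.
; Later interactions use a FlipFlop to alternately hide and show the cached widget, switching cursor and input mode to match.
; Without the flag, it only prints "NieMoznaBezGazety" (not possible without the newspaper).
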(event `self.BeginInteraction`
  (bind _returnvalue (`GameplayStatics.GetPlayerController` 0))
  (bind _returnvalue_2 (`GameplayStatics.GetPlayerController` 0))
  (bind _level_3_glosnik (`self.Level 3 Glosnik`))
  (`parent.BeginInteraction`)
  (bind _asbp_first_person_character (cast `/Game/FirstPerson/Blueprints/BP_FirstPersonCharacter` (`GameplayStatics.GetPlayerCharacter` 0)))
  (if (`/Game/FirstPerson/Blueprints/BP_FirstPersonCharacter.Level3_Interacted` _asbp_first_person_character)
    (`self.Level 3 Glosnik`
      (:`then`
        (`/Engine/EditorBlueprintResources/StandardMacros.FlipFlop`
          (:`A`
            (`Widget.SetVisibility` _level_3_glosnik "Hidden")
            (set `PlayerController.bShowMouseCursor` false _returnvalue)
            (`WidgetBlueprintLibrary.SetInputMode_GameOnly` _returnvalue))
          (:`B`
            (`Widget.SetVisibility` _level_3_glosnik "Visible")
            (set `PlayerController.bShowMouseCursor` true _returnvalue)
            (`WidgetBlueprintLibrary.SetInputMode_GameAndUIEx` _returnvalue_2 null :!label _label))))
      (:`else`
        (bind _returnvalue_3 (`|CreateWidget` "/Game/LevelWidgets/Level3/WB_Level3_Glosnik.WB_Level3_Glosnik_C" (`GameplayStatics.GetPlayerController` 0)))
        (bind _output_get (set `self.Level 3 Glosnik` _returnvalue_3))
        (`UserWidget.AddToViewport` _output_get 0)
        (`Widget.SetVisibility` (`self.Level 3 Glosnik`) "Visible")
        (set `PlayerController.bShowMouseCursor` true _returnvalue_2)
        (goto _label)))
    (else
      (`KismetSystemLibrary.PrintText` "NieMoznaBezGazety"))))

(fn `UserConstructionScript`
  (`parent.UserConstructionScript`))