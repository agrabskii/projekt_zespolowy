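; BP_Makieta is an interactable in Level 1 that toggles a close-up view with cables on each interaction.
; A FlipFlop on BeginInteraction alternates between entering and leaving the view.
; Entering sends the player character a fixed camera pose, shows and enables collision on Cables, and turns on the cursor with game-and-UI input.
; Leaving restores the camera, hides and disables the cables, and returns to game-only input.
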(event `self.BeginInteraction`
  (bind _returnvalue (`GameplayStatics.GetPlayerCharacter` 0))
  (bind _returnvalue_2 (`GameplayStatics.GetPlayerController` 0))
  (bind _cables (`self.Cables`))
  ; Interaction
  (`/Engine/EditorBlueprintResources/StandardMacros.FlipFlop`
    (:`A`
      (message `/Game/Interactions/BPI_Interaction.Camera_Adjust_On` _returnvalue (`KismetMathLibrary.MakeVector` 194.140054 240.0 150.0) (`KismetMathLibrary.MakeRotator` 0.0 -90.0))
      (`SceneComponent.SetVisibility` _cables true false)
      (set `PlayerController.bShowMouseCursor` true _returnvalue_2)
      (`WidgetBlueprintLibrary.SetInputMode_GameAndUIEx` _returnvalue_2 null "DoNotLock" false)
      (`PrimitiveComponent.SetCollisionEnabled` _cables "QueryAndPhysics"))
    (:`B`
      (message `/Game/Interactions/BPI_Interaction.Camera_Adjust_Off` _returnvalue)
      (`SceneComponent.SetVisibility` _cables false false)
      (set `PlayerController.bShowMouseCursor` false _returnvalue_2)
      (`WidgetBlueprintLibrary.SetInputMode_GameOnly` _returnvalue_2)
      (`PrimitiveComponent.SetCollisionEnabled` _cables "NoCollision"))))

(fn `UserConstructionScript`)