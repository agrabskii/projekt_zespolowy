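; BP_Monitor6 is an interactable Level 6 monitor that shows Polish number-riddle clues across three widget-component screens.
; BeginInteraction flip-flops between an adjusted camera with mouse input and normal play, and the first screen's Exit button reuses it.
; Buttons move between screens by swapping visibility and collision while tracking CurrentWidget.
; PIN buttons set the third screen's riddle text, one varying with BP_Komputer6's PendriveIn flag.
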(event `Exit`
  (`self.BeginInteraction`))

(event `Part1_Next`
  (bind _part2 (`self.Part2`))
  (bind _part1 (`self.Part1`))
  (`SceneComponent.SetVisibility` _part1 false false)
  (`PrimitiveComponent.SetCollisionEnabled` _part1 "NoCollision")
  (`SceneComponent.SetVisibility` _part2 true false)
  (`PrimitiveComponent.SetCollisionEnabled` _part2 "QueryOnly")
  (set `self.Current_Widget` _part2))

(event `self.ReceiveBeginPlay`
  (bind _part1 (`self.Part1`))
  (`|ExecutionSequence`
    (:`then_0`
      (`PrimitiveComponent.SetCollisionEnabled` (`self.Part2`) "NoCollision")
      (`PrimitiveComponent.SetCollisionEnabled` (`self.Part3`) "NoCollision")
      (bind _aswbp_lvl_10_2 (cast `/Game/Levels/Level_6/Components/WBP_Lvl10_2` (`WidgetComponent.GetWidget` _part1)))
      (add `Button.OnClicked` (`/Game/Levels/Level_6/Components/WBP_Lvl10_2.Exit_Button` _aswbp_lvl_10_2) (delegate `Exit`))
      (add `Button.OnClicked` (`/Game/Levels/Level_6/Components/WBP_Lvl10_2.Next_Button` _aswbp_lvl_10_2) (delegate `Part1_Next`))
      (set `self.Current_Widget` _part1))
    (:`then_1`
      (bind _aswbp_lvl_10_21 (cast `/Game/Levels/Level_6/Components/WBP_Lvl10_21` (`WidgetComponent.GetWidget` (`self.Part2`))))
      (add `Button.OnClicked` (`/Game/Levels/Level_6/Components/WBP_Lvl10_21.Exit_Button` _aswbp_lvl_10_21) (delegate `Part2_Back`))
      (add `Button.OnClicked` (`/Game/Levels/Level_6/Components/WBP_Lvl10_21.PIN_Button` _aswbp_lvl_10_21) (delegate `2Question`))
      (add `Button.OnClicked` (`/Game/Levels/Level_6/Components/WBP_Lvl10_21.PIN_Button_1` _aswbp_lvl_10_21) (delegate `4Question`)))
    (:`then_2`
      (bind _aswbp_lvl_10_22 (cast `/Game/Levels/Level_6/Components/WBP_Lvl10_22` (`WidgetComponent.GetWidget` (`self.Part3`))))
      (add `Button.OnClicked` (`/Game/Levels/Level_6/Components/WBP_Lvl10_22.Exit_Button` _aswbp_lvl_10_22) (delegate `Part3_Back`)))))

(event `Part2_Back`
  (bind _part1 (`self.Part1`))
  (bind _part2 (`self.Part2`))
  (`SceneComponent.SetVisibility` _part2 false false)
  (`PrimitiveComponent.SetCollisionEnabled` _part2 "NoCollision")
  (`SceneComponent.SetVisibility` _part1 true false)
  (`PrimitiveComponent.SetCollisionEnabled` _part1 "QueryOnly")
  (set `self.Current_Widget` _part1))

(event `4Question`
  (`self.Part2_Next`)
  (bind _returnvalue (`GameplayStatics.GetActorOfClass` "/Game/Levels/Level_6/BP_Komputer6.BP_Komputer6_C"))
  (if (`/Game/Levels/Level_6/BP_Komputer6.PendriveIn?` _returnvalue)
    (bind _text_var (`/Game/Levels/Level_6/Components/WBP_Lvl10_22.Text_Var` (stale `self.ReceiveBeginPlay` _aswbp_lvl_10_22)))
    (`TextBlock.SetText` _text_var "„Suma liczb: 7, ?, 5, 9 wynosi 27”")
    (else
      (`TextBlock.SetText` _text_var "Liczba 2:                                                                                                                            „Jaka to liczba? Dzieli się przez 3(? nie 2?) i 4 nie dzieli się przez 6 jest mniejsza niż 20”"))))

(event `2Question`
  (`self.Part2_Next`)
  (`TextBlock.SetText` (`/Game/Levels/Level_6/Components/WBP_Lvl10_22.Text_Var` (stale `self.ReceiveBeginPlay` _aswbp_lvl_10_22)) "Liczba 2:                                                                                                                            „Jaka to liczba? Dzieli się przez 3(? nie 2?) i 4 nie dzieli się przez 6 jest mniejsza niż 20”"))

(event `Part2_Next`
  (bind _part3 (`self.Part3`))
  (bind _part2 (`self.Part2`))
  (`SceneComponent.SetVisibility` _part3 true false)
  (`PrimitiveComponent.SetCollisionEnabled` _part3 "QueryAndPhysics")
  (`SceneComponent.SetVisibility` _part2 false false)
  (`PrimitiveComponent.SetCollisionEnabled` _part2 "NoCollision")
  (set `self.Current_Widget` _part3))

(event `Part3_Back`
  (bind _part3 (`self.Part3`))
  (bind _part2 (`self.Part2`))
  (`SceneComponent.SetVisibility` _part3 false false)
  (`PrimitiveComponent.SetCollisionEnabled` _part3 "NoCollision")
  (`SceneComponent.SetVisibility` _part2 true false)
  (`PrimitiveComponent.SetCollisionEnabled` _part2 "QueryOnly")
  (set `self.Current_Widget` _part2))

(event `self.BeginInteraction`
  (bind _returnvalue (`GameplayStatics.GetPlayerCharacter` 0))
  (bind _returnvalue_2 (`GameplayStatics.GetPlayerController` 0))
  (bind _current_widget (`self.Current_Widget`))
  (`/Engine/EditorBlueprintResources/StandardMacros.FlipFlop`
    (:`A`
      (message `/Game/Interactions/BPI_Interaction.Camera_Adjust_On` _returnvalue (`KismetMathLibrary.MakeVector` 219.686055 -125.538621 149.66165) (`KismetMathLibrary.MakeRotator` 0.0 -5.0 0.0))
      (set `PlayerController.bShowMouseCursor` true _returnvalue_2)
      (`WidgetBlueprintLibrary.SetInputMode_GameAndUIEx` _returnvalue_2 null "DoNotLock" false)
      (`SceneComponent.SetVisibility` _current_widget true false))
    (:`B`
      (message `/Game/Interactions/BPI_Interaction.Camera_Adjust_Off` _returnvalue)
      (set `PlayerController.bShowMouseCursor` false _returnvalue_2)
      (`WidgetBlueprintLibrary.SetInputMode_GameOnly` _returnvalue_2)
      (`SceneComponent.SetVisibility` _current_widget false false)
      (`PrimitiveComponent.SetCollisionEnabled` (`self.Current_Widget`) "NoCollision")
      (if (`self.WinInstalled?`)
        (bind _output_get (set `self.Current_Widget` null))
        (`PrimitiveComponent.SetCollisionEnabled` _output_get "QueryOnly")
        (else
          (bind _output_get_2 (set `self.Current_Widget` (`self.Part1`)))
          (`PrimitiveComponent.SetCollisionEnabled` _output_get_2 "QueryOnly"))))))

(fn `UserConstructionScript`)