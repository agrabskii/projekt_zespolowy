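; BP_Szafka is an interactable cabinet in Level 6 that responds only after the BP_Klucz6 key has been picked up.
; Successive BeginInteraction calls first rotate the door open, then move the BP_Paper6 child actor to a new relative location, then forward interaction to that paper.
; The Open and OnTop flags track the stage, and both movements are instant transform changes without animation.
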(event `self.BeginInteraction`
  (bind _bp_paper6 (`self.BP_Paper6`))
  (bind _returnvalue (`GameplayStatics.GetActorOfClass` "/Game/Levels/Level_6/BP_Klucz6.BP_Klucz6_C"))
  (if (`/Game/Levels/Level_6/BP_Klucz6.PickedUp?` _returnvalue)
    (if (`self.OnTop?`)
      (bind _asbp_paper_6 (cast `/Game/Levels/Level_6/BP_Paper6` (`ChildActorComponent.ChildActor` _bp_paper6)))
      (`self.BeginInteraction` _asbp_paper_6)
      (elif (`self.Open?`)
        (`SceneComponent.K2_SetRelativeLocation` _bp_paper6 (0.0 0.0 369.486009) false false)
        (set `self.OnTop?` true)
        (else
          (`SceneComponent.K2_SetRelativeRotation` (`self.drzwiczki-szafki`) (struct :`Yaw` -20.0) false false)
          (set `self.Open?` true))))))

(fn `UserConstructionScript`)