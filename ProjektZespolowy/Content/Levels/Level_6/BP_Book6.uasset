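; BP_Book6 is an interactable book for Level 6 that toggles a close-up reading view.
; BeginInteraction uses a FlipFlop: the first call moves the player camera to a hard-coded top-down position, shows the cursor, switches to game-and-UI input and reveals the Zad1 component with collision enabled.
; The next call restores the camera and game-only input, hides the cursor and Zad1, and disables its collision.
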(event `self.BeginInteraction`
  (bind _returnvalue (`GameplayStatics.GetPlayerCharacter` 0))
  (bind _returnvalue_2 (`GameplayStatics.GetPlayerController` 0))
  (bind _zad_1 (`self.Zad_1`))
  (`/Engine/EditorBlueprintResources/StandardMacros.FlipFlop`
    (:`A`
      (message `/Game/Interactions/BPI_Interaction.Camera_Adjust_On` _returnvalue (`KismetMathLibrary.MakeVector` 19.671228 309.876905 162.510764) (`KismetMathLibrary.MakeRotator` 0.0 -90.0 90.0))
      (set `PlayerController.bShowMouseCursor` true _returnvalue_2)
      (`WidgetBlueprintLibrary.SetInputMode_GameAndUIEx` _returnvalue_2 null "DoNotLock" false)
      (`SceneComponent.SetVisibility` _zad_1 true false)
      (`PrimitiveComponent.SetCollisionEnabled` _zad_1 "QueryAndPhysics"))
    (:`B`
      (message `/Game/Interactions/BPI_Interaction.Camera_Adjust_Off` _returnvalue)
      (set `PlayerController.bShowMouseCursor` false _returnvalue_2)
      (`WidgetBlueprintLibrary.SetInputMode_GameOnly` _returnvalue_2)
      (`SceneComponent.SetVisibility` _zad_1 false false)
      (`PrimitiveComponent.SetCollisionEnabled` _zad_1 "NoCollision"))))

(fn `UserConstructionScript`
  (`parent.UserConstructionScript`))