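; BPC_Level6 is a Level 6 component that pre-creates UI widgets, apparently for the level's puzzles ("Zagadka").
; On BeginPlay it creates WBP_1, WBP_Lvl10_2 and WBP_3, adds each to the viewport hidden and stores them in Zagadka1, Windows1 and Zagadka3.
; It contains no logic to show the widgets, and Tick is unused.
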(event `self.ReceiveBeginPlay`
  (bind _returnvalue (`|CreateWidget` "/Game/Levels/Level_6/Components/WBP_1.WBP_1_C"))
  (bind _output_get (set `self.Zagadka1` _returnvalue))
  (`UserWidget.AddToViewport` _output_get 0)
  (`Widget.SetVisibility` _output_get "Hidden")
  (bind _returnvalue_2 (`|CreateWidget` "/Game/Levels/Level_6/Components/WBP_Lvl10_2.WBP_Lvl10_2_C"))
  (bind _output_get_2 (set `self.Windows1` _returnvalue_2))
  (`UserWidget.AddToViewport` _output_get_2 0)
  (`Widget.SetVisibility` _output_get_2 "Hidden")
  (bind _returnvalue_3 (`|CreateWidget` "/Game/Levels/Level_6/Components/WBP_3.WBP_3_C"))
  (bind _output_get_3 (set `self.Zagadka 3` _returnvalue_3))
  (`UserWidget.AddToViewport` _output_get_3 0)
  (`Widget.SetVisibility` _output_get_3 "Hidden"))