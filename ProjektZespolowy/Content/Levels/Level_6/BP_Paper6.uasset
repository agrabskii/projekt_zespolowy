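; BP_Paper6 is an interactable paper in Level 6 that presents a question widget (3Question) to the first-person player.
; BeginInteraction uses a FlipFlop to toggle between a focused view and normal play.
; Focusing sends a camera-adjust message with a hardcoded transform, shows the question with collision enabled, and switches to mouse cursor with Game and UI input.
; The next interaction reverses all of it.
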(event `self.BeginInteraction`
  (bind _returnvalue (`GameplayStatics.GetPlayerCharacter` 0))
  (bind _returnvalue_2 (`GameplayStatics.GetPlayerController` 0))
  (bind _3question (`self.3Question`))
  (cast `/Game/FirstPerson/Blueprints/BP_FirstPersonCharacter` _returnvalue)
  (`/Engine/EditorBlueprintResources/StandardMacros.FlipFlop`
    (:`A`
      (message `/Game/Interactions/BPI_Interaction.Camera_Adjust_On` _returnvalue (`KismetMathLibrary.MakeVector` 193.991782 457.781552 140.179979) (`KismetMathLibrary.MakeRotator` 90.0 -90.0))
      (`SceneComponent.SetVisibility` _3question true false)
      (set `PlayerController.bShowMouseCursor` true _returnvalue_2)
      (`WidgetBlueprintLibrary.SetInputMode_GameAndUIEx` _returnvalue_2 null "DoNotLock" false)
      (`PrimitiveComponent.SetCollisionEnabled` _3question "QueryAndPhysics"))
    (:`B`
      (message `/Game/Interactions/BPI_Interaction.Camera_Adjust_Off` _returnvalue)
      (`SceneComponent.SetVisibility` _3question false false)
      (set `PlayerController.bShowMouseCursor` false _returnvalue_2)
      (`WidgetBlueprintLibrary.SetInputMode_GameOnly` _returnvalue_2)
      (`PrimitiveComponent.SetCollisionEnabled` _3question "NoCollision"))))

(fn `UserConstructionScript`)