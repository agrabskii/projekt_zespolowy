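; Interactable combination padlock for Level 6 that opens a code-entry UI when the player interacts with it.
; BeginPlay creates a WBP_Lock widget, and SetOdp forwards four answers and a level class to it.
; Each interaction flip-flops between showing the widget with mouse cursor, Game and UI input and movement disabled, and hiding it with game-only input and walking restored.
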(event `SetOdp`
  (params (Odp1 :type String) (Odp2 :type String) (Odp3 :type String) (Odp4 :type String) (LevelClass :type "Actor Class Reference"))
  (`/Game/Levels/Level_6/WBP_Lock.SetOdp` (`self.WBP_Lock`) Odp1 Odp2 Odp3 Odp4 LevelClass))

(event `self.ReceiveBeginPlay`
  (bind _returnvalue (`|CreateWidget` "/Game/Levels/Level_6/WBP_Lock.WBP_Lock_C" (`GameplayStatics.GetPlayerController` 0)))
  (set `self.WBP_Lock` _returnvalue))

(event `self.BeginInteraction`
  (bind _returnvalue (`GameplayStatics.GetPlayerController` 0))
  (bind _returnvalue_2 (`GameplayStatics.GetPlayerController` 0))
  (bind _charactermovement (`Character.CharacterMovement` (`GameplayStatics.GetPlayerCharacter` 0)))
  (`parent.BeginInteraction`)
  (`/Engine/EditorBlueprintResources/StandardMacros.FlipFlop`
    (:`A`
      (`UserWidget.AddToViewport` (`self.WBP_Lock`) 0)
      (`Widget.SetVisibility` (`self.WBP_Lock`) "Visible")
      (set `PlayerController.bShowMouseCursor` true _returnvalue)
      (`WidgetBlueprintLibrary.SetInputMode_GameAndUIEx` _returnvalue null "DoNotLock" false)
      (`CharacterMovementComponent.DisableMovement` _charactermovement))
    (:`B`
      (`Widget.SetVisibility` (`self.WBP_Lock`) "Hidden")
      (set `PlayerController.bShowMouseCursor` false _returnvalue_2)
      (`WidgetBlueprintLibrary.SetInputMode_GameOnly` _returnvalue_2)
      (`CharacterMovementComponent.SetMovementMode` _charactermovement "MOVE_Walking" 0))))

(fn `UserConstructionScript`)