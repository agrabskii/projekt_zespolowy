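; Level 8 interactive monitor that simulates a Linux and Windows computer, including file screens with PIN puzzle clues.
; BeginInteraction uses a FlipFlop to enter or leave a fixed camera with cursor input; top-level Exit buttons call it again.
; Widget button bindings page between screens by toggling visibility and collision, tracking CurrentWidget.
; A pendrive in BP_Komputer8 brings up Windows, whose Next button marks it installed, changing the resume screen.
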(event `Exit`
  (`self.BeginInteraction`))

(event `Lin1_Next`
  (bind _linux_2 (`self.Linux_2`))
  (bind _linux_1 (`self.Linux_1`))
  (`SceneComponent.SetVisibility` _linux_1 false false)
  (`PrimitiveComponent.SetCollisionEnabled` _linux_1 "NoCollision")
  (`SceneComponent.SetVisibility` _linux_2 true false)
  (`PrimitiveComponent.SetCollisionEnabled` _linux_2 "QueryOnly")
  (set `self.Current_Widget` _linux_2))

(event `Lin2_Back`
  (bind _linux_1 (`self.Linux_1`))
  (bind _linux_2 (`self.Linux_2`))
  (`SceneComponent.SetVisibility` _linux_2 false false)
  (`PrimitiveComponent.SetCollisionEnabled` _linux_2 "NoCollision")
  (`SceneComponent.SetVisibility` _linux_1 true false)
  (`PrimitiveComponent.SetCollisionEnabled` _linux_1 "QueryOnly")
  (set `self.Current_Widget` _linux_1))

(event `Lin2_Next`
  (bind _linux_3 (`self.Linux_3`))
  (bind _linux_2 (`self.Linux_2`))
  (`SceneComponent.SetVisibility` _linux_2 false false)
  (`PrimitiveComponent.SetCollisionEnabled` _linux_2 "NoCollision")
  (`SceneComponent.SetVisibility` _linux_3 true false)
  (`PrimitiveComponent.SetCollisionEnabled` _linux_3 "QueryOnly")
  (set `self.Current_Widget` _linux_3))

(event `Lin3_Back`
  (bind _linux_3 (`self.Linux_3`))
  (bind _linux_2 (`self.Linux_2`))
  (`SceneComponent.SetVisibility` _linux_3 false false)
  (`PrimitiveComponent.SetCollisionEnabled` _linux_3 "NoCollision")
  (`SceneComponent.SetVisibility` _linux_2 true false)
  (`PrimitiveComponent.SetCollisionEnabled` _linux_2 "QueryOnly")
  (set `self.Current_Widget` _linux_2))

(event `self.ReceiveBeginPlay`
  (bind _linux_1 (`self.Linux_1`))
  (`|ExecutionSequence`
    (:`then_0`
      (`PrimitiveComponent.SetCollisionEnabled` (`self.Linux_2`) "NoCollision")
      (`PrimitiveComponent.SetCollisionEnabled` (`self.Linux_3`) "NoCollision")
      (`PrimitiveComponent.SetCollisionEnabled` (`self.Win_1`) "NoCollision")
      (`PrimitiveComponent.SetCollisionEnabled` (`self.Win_2`) "NoCollision")
      (`PrimitiveComponent.SetCollisionEnabled` (`self.Win_3`) "NoCollision")
      (`PrimitiveComponent.SetCollisionEnabled` (`self.Win_4`) "NoCollision")
      (bind _aswbp_system_linux (cast `/Game/Levels/Level_8/Linux/WBP_SystemLinux` (`WidgetComponent.GetWidget` _linux_1)))
      (add `Button.OnClicked` (`/Game/Levels/Level_8/Linux/WBP_SystemLinux.Exit_Button` _aswbp_system_linux) (delegate `Exit`))
      (add `Button.OnClicked` (`/Game/Levels/Level_8/Linux/WBP_SystemLinux.Next_Button` _aswbp_system_linux) (delegate `Lin1_Next`))
      (set `self.Current_Widget` _linux_1))
    (:`then_1`
      (bind _aswbp_system_linux_1 (cast `/Game/Levels/Level_8/Linux/WBP_SystemLinux1` (`WidgetComponent.GetWidget` (`self.Linux_2`))))
      (add `Button.OnClicked` (`/Game/Levels/Level_8/Linux/WBP_SystemLinux1.Exit_Button` _aswbp_system_linux_1) (delegate `Lin2_Back`))
      (add `Button.OnClicked` (`/Game/Levels/Level_8/Linux/WBP_SystemLinux1.Next_Button` _aswbp_system_linux_1) (delegate `Lin2_Next`)))
    (:`then_2`
      (bind _aswbp_system_linux_2 (cast `/Game/Levels/Level_8/Linux/WBP_SystemLinux2` (`WidgetComponent.GetWidget` (`self.Linux_3`))))
      (add `Button.OnClicked` (`/Game/Levels/Level_8/Linux/WBP_SystemLinux2.Exit_Button` _aswbp_system_linux_2) (delegate `Lin3_Back`)))
    (:`then_3`
      (bind _aswbp_windows_1 (cast `/Game/Levels/Level_8/WIndows/WBP_Windows1` (`WidgetComponent.GetWidget` (`self.Win_1`))))
      (add `Button.OnClicked` (`/Game/Levels/Level_8/WIndows/WBP_Windows1.Exit_Button` _aswbp_windows_1) (delegate `Exit`))
      (add `Button.OnClicked` (`/Game/Levels/Level_8/WIndows/WBP_Windows1.Next_Button` _aswbp_windows_1) (delegate `Win1_Next`)))
    (:`then_4`
      (bind _aswbp_windows_2 (cast `/Game/Levels/Level_8/WIndows/WBP_Windows2` (`WidgetComponent.GetWidget` (`self.Win_2`))))
      (add `Button.OnClicked` (`/Game/Levels/Level_8/WIndows/WBP_Windows2.Exit_Button` _aswbp_windows_2) (delegate `Exit`))
      (add `Button.OnClicked` (`/Game/Levels/Level_8/WIndows/WBP_Windows2.Next_Button` _aswbp_windows_2) (delegate `Win2_Next`)))
    (:`then_5`
      (bind _aswbp_windows_3 (cast `/Game/Levels/Level_8/WIndows/WBP_Windows3` (`WidgetComponent.GetWidget` (`self.Win_3`))))
      (add `Button.OnClicked` (`/Game/Levels/Level_8/WIndows/WBP_Windows3.Exit_Button` _aswbp_windows_3) (delegate `Win3_Back`))
      (bind _aswbp_windows_4 (cast `/Game/Levels/Level_8/WIndows/WBP_Windows4` (`WidgetComponent.GetWidget` (`self.Win_4`))))
      (add `Button.OnClicked` (`/Game/Levels/Level_8/WIndows/WBP_Windows3.PIN_Button` _aswbp_windows_3) (delegate `PIN`))
      (add `Button.OnClicked` (`/Game/Levels/Level_8/WIndows/WBP_Windows3.SL_Button` _aswbp_windows_3) (delegate `SL`))
      (add `Button.OnClicked` (`/Game/Levels/Level_8/WIndows/WBP_Windows3.U_Button` _aswbp_windows_3) (delegate `U`))
      (add `Button.OnClicked` (`/Game/Levels/Level_8/WIndows/WBP_Windows3.Zad_Button` _aswbp_windows_3) (delegate `Zad`)))
    (:`then_6`
      (bind _aswbp_windows_4_2 (cast `/Game/Levels/Level_8/WIndows/WBP_Windows4` (`WidgetComponent.GetWidget` (`self.Win_4`))))
      (add `Button.OnClicked` (`/Game/Levels/Level_8/WIndows/WBP_Windows4.Exit_Button` _aswbp_windows_4_2) (delegate `Win4_Back`)))))

(event `Win1_Next`
  (bind _win_2 (`self.Win_2`))
  (bind _win_1 (`self.Win_1`))
  (set `self.WinInstalled?` true)
  (`SceneComponent.SetVisibility` _win_1 false false)
  (`PrimitiveComponent.SetCollisionEnabled` _win_1 "NoCollision")
  (`SceneComponent.SetVisibility` _win_2 true false)
  (`PrimitiveComponent.SetCollisionEnabled` _win_2 "QueryOnly")
  (set `self.Current_Widget` _win_2))

(event `Win2_Next`
  (bind _win_3 (`self.Win_3`))
  (bind _win_2 (`self.Win_2`))
  (`SceneComponent.SetVisibility` _win_2 false false)
  (`PrimitiveComponent.SetCollisionEnabled` _win_2 "NoCollision")
  (`SceneComponent.SetVisibility` _win_3 true false)
  (`PrimitiveComponent.SetCollisionEnabled` _win_3 "QueryOnly")
  (set `self.Current_Widget` _win_3))

(event `Win3_Back`
  (bind _win_3 (`self.Win_3`))
  (bind _win_2 (`self.Win_2`))
  (`SceneComponent.SetVisibility` _win_3 false false)
  (`PrimitiveComponent.SetCollisionEnabled` _win_3 "NoCollision")
  (`SceneComponent.SetVisibility` _win_2 true false)
  (`PrimitiveComponent.SetCollisionEnabled` _win_2 "QueryOnly")
  (set `self.Current_Widget` _win_2))

(event `PIN`
  (`self.Show_Win4`)
  (`TextBlock.SetText` (`/Game/Levels/Level_8/WIndows/WBP_Windows4.Text_Var` (stale `self.ReceiveBeginPlay` _aswbp_windows_4)) "PIN -> (L)ID USER | (L)FILE SIZE | (L)FILE DATE |  ZAD.TXT LETTER COUNT"))

(event `SL`
  (`self.Show_Win4`)
  (`TextBlock.SetText` (`/Game/Levels/Level_8/WIndows/WBP_Windows4.Text_Var` (stale `self.ReceiveBeginPlay` _aswbp_windows_4)) "data encrypted! Size: 236 KB"))

(event `U`
  (`self.Show_Win4`)
  (`TextBlock.SetText` (`/Game/Levels/Level_8/WIndows/WBP_Windows4.Text_Var` (stale `self.ReceiveBeginPlay` _aswbp_windows_4)) "1. user105"))

(event `Zad`
  (`self.Show_Win4`)
  (`TextBlock.SetText` (`/Game/Levels/Level_8/WIndows/WBP_Windows4.Text_Var` (stale `self.ReceiveBeginPlay` _aswbp_windows_4)) "Data enc... 15.04.2024"))

(event `Show_Win4`
  (bind _win_4 (`self.Win_4`))
  (bind _win_3 (`self.Win_3`))
  (`SceneComponent.SetVisibility` _win_3 false false)
  (`PrimitiveComponent.SetCollisionEnabled` _win_3 "NoCollision")
  (`SceneComponent.SetVisibility` _win_4 true false)
  (`PrimitiveComponent.SetCollisionEnabled` _win_4 "QueryOnly")
  (set `self.Current_Widget` _win_4))

(event `Win4_Back`
  (bind _win_3 (`self.Win_3`))
  (bind _win_4 (`self.Win_4`))
  (`SceneComponent.SetVisibility` _win_4 false false)
  (`PrimitiveComponent.SetCollisionEnabled` _win_4 "NoCollision")
  (`SceneComponent.SetVisibility` _win_3 true false)
  (`PrimitiveComponent.SetCollisionEnabled` _win_3 "QueryOnly")
  (set `self.Current_Widget` _win_3))

(event `self.BeginInteraction`
  (bind _returnvalue (`GameplayStatics.GetPlayerCharacter` 0))
  (bind _returnvalue_2 (`GameplayStatics.GetPlayerController` 0))
  (bind _current_widget (`self.Current_Widget`))
  (bind _win_1 (`self.Win_1`))
  (bind _returnvalue_3 (`GameplayStatics.GetActorOfClass` "/Game/Levels/Level_8/BP_Komputer8.BP_Komputer8_C"))
  (if (and (not (`self.WinInstalled?`)) (`/Game/Levels/Level_8/BP_Komputer8.PnedriveIn?` _returnvalue_3))
    (`SceneComponent.SetVisibility` _win_1 true false)
    (`PrimitiveComponent.SetCollisionEnabled` _win_1 "QueryOnly")
    (set `self.Current_Widget` _win_1))
  (`/Engine/EditorBlueprintResources/StandardMacros.FlipFlop`
    (:`A`
      (message `/Game/Interactions/BPI_Interaction.Camera_Adjust_On` _returnvalue (`KismetMathLibrary.MakeVector` 257.650106 715.683307 156.941589) (`KismetMathLibrary.MakeRotator` 0.0 -5.0 180.0))
      (set `PlayerController.bShowMouseCursor` true _returnvalue_2)
      (`WidgetBlueprintLibrary.SetInputMode_GameAndUIEx` _returnvalue_2 null "DoNotLock" false)
      (`SceneComponent.SetVisibility` _current_widget true false))
    (:`B`
      (message `/Game/Interactions/BPI_Interaction.Camera_Adjust_Off` _returnvalue)
      (set `PlayerController.bShowMouseCursor` false _returnvalue_2)
      (`WidgetBlueprintLibrary.SetInputMode_GameOnly` _returnvalue_2)
      (`SceneComponent.SetVisibility` _current_widget false false)
      (`PrimitiveComponent.SetCollisionEnabled` (`self.Current_Widget`) "NoCollision")
      (if (`self.WinInstalled?`)
        (bind _output_get (set `self.Current_Widget` (`self.Win_2`)))
        (`PrimitiveComponent.SetCollisionEnabled` _output_get "QueryOnly")
        (else
          (bind _output_get_2 (set `self.Current_Widget` (`self.Linux_1`)))
          (`PrimitiveComponent.SetCollisionEnabled` _output_get_2 "QueryOnly"))))))

(fn `UserConstructionScript`)