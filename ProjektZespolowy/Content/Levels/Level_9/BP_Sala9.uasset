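; BP_Sala9 is the room Blueprint for Level 9 that handles the exit to Level 10.
; A SetPassable event casts the BPDoor child actor to BP_Door and calls PassTrue on it.
; Tick polls DoorOpen, which is not set in these graphs, and when true opens L_Level10, hides the mouse cursor and switches to game-only input.
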(event `self.ReceiveTick`
  (params (DeltaSeconds :type "Float (single-precision)"))
  (bind _returnvalue (`GameplayStatics.GetPlayerController` 0))
  (if (`self.DoorOpen`)
    (`GameplayStatics.OpenLevelBySoftObjectPtr` "/Game/Levels/Level_10/L_Level10.L_Level10")
    (set `PlayerController.bShowMouseCursor` false _returnvalue)
    (`WidgetBlueprintLibrary.SetInputMode_GameOnly` _returnvalue)))

(event `SetPassable`
  (bind _asbp_door (cast `/Game/Levels/Items/Doors/BP_Door` (`ChildActorComponent.ChildActor` (`self.BP_Door`))))
  (`/Game/Levels/Items/Doors/BP_Door.PassTrue` _asbp_door))

(fn `UserConstructionScript`)