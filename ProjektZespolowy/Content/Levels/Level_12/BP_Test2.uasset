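; BP_Test2 is an interactable Level 12 actor that toggles the WB_Level12_Test2 widget on screen.
; The first interaction creates and stores the widget, adds it to the viewport, shows the cursor and sets Game and UI input.
; Later interactions use a FlipFlop to alternately hide and show that widget, switching cursor visibility and input mode between Game Only and Game and UI.
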(event `self.BeginInteraction`
  (bind _returnvalue (`GameplayStatics.GetPlayerController` 0))
  (bind _returnvalue_2 (`GameplayStatics.GetPlayerController` 0))
  (bind _level12part2 (`self.Level12Part2`))
  (`parent.BeginInteraction`)
  (`self.Level12Part2`
    (:`then`
      (`/Engine/EditorBlueprintResources/StandardMacros.FlipFlop`
        (:`A`
          (`Widget.SetVisibility` _level12part2 "Hidden")
          (set `PlayerController.bShowMouseCursor` false _returnvalue)
          (`WidgetBlueprintLibrary.SetInputMode_GameOnly` _returnvalue))
        (:`B`
          (`Widget.SetVisibility` _level12part2 "Visible")
          (set `PlayerController.bShowMouseCursor` true _returnvalue)
          (`WidgetBlueprintLibrary.SetInputMode_GameAndUIEx` _returnvalue_2 null :!label _label))))
    (:`else`
      (bind _returnvalue_3 (`|CreateWidget` "/Game/LevelWidgets/Level12/WB_Level12_Test2.WB_Level12_Test2_C" (`GameplayStatics.GetPlayerController` 0)))
      (bind _output_get (set `self.Level12Part2` _returnvalue_3))
      (`UserWidget.AddToViewport` _output_get 0)
      (`Widget.SetVisibility` (`self.Level12Part2`) "Visible")
      (set `PlayerController.bShowMouseCursor` true _returnvalue_2)
      (goto _label))))

(fn `UserConstructionScript`
  (`parent.UserConstructionScript`))